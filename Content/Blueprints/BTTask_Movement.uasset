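; Behavior tree task that sets an AI's TargetPoint to the building named by its Route blackboard key.
; On execute it loops over all Building actors, matches BuildingName, and writes the capsule's nav-projected location to the blackboard, then finishes successfully.
; It disables the owner's collision if the matched capsule lies near world origin, not near the owner.
; A debug print and an unreachable fallback target remain.
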(event EventReceiveExecute
  (params (OwnerActor :type Actor%20Object%20Reference))
  ;[1 1 1] Update TargetPoint to NextRoute
  (bind _outactors (Actor|GetAllActorsOfClass "/Game/Blueprints/Building.Building_C"))
  (bind _array_element (Utilities|Array|ForEachLoopwithBreak _outactors)
    (:LoopBody
      (bind _asbuilding (Utilities|Casting|CastToBuilding _array_element))
      (Development|PrintString (Utilities|String|ToString(Vector) "0, 0, 0"))
      (if (Utilities|Name|Equal(Name) (Variables|/Game/Blueprints/Building.Building_C|GetBuildingName _asbuilding) (Class|BTFunctionLibrary|GetBlackboardValueasName (Variables|Default|GetRoute)))
        (AI|BehaviorTree|SetBlackboardValueasVector (Variables|Default|GetTargetPoint) (AI|Navigation|ProjectPointtoNavigation (Transformation|GetWorldLocation (Variables|/Game/Blueprints/Building.Building_C|GetCapsule _asbuilding)) 0 0))
        (if (Math|Vector|Equal(Vector) "0, 0, 0" (Transformation|GetWorldLocation (Variables|/Game/Blueprints/Building.Building_C|GetCapsule _asbuilding)) 5e+01)
          (Collision|SetActorEnableCollision OwnerActor false))))
    (:Completed
      (AI|BehaviorTree|FinishExecute true))))