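; AI Controller that wanders its pawn around the navmesh and spreads a disease between AI characters.
; Each Tick requests a move toward a random reachable-radius destination, re-picked when the move fails or is already at goal.
; It then sphere-overlaps nearby AI within DiseaseRadius, infecting its own pawn if a neighbour is infected.
; Infection attaches a disease particle, also shown on BeginPlay for initially infected pawns; behavior tree startup is disconnected.
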(event EventTick
  (params (DeltaSeconds :type Float%20%28single-precision%29))
  (CallFunction|MovetoRandomLocation (stale EventBeginPlay _array_element))
  (bind _location (CallFunction|GetCharacterLocation))
  (bind (_outactors _returnvalue) (Class|KismetSystemLibrary|SphereOverlapActorsNEW _location (Variables|Default|GetDiseaseRadius) (Utilities|Array|MakeArray "ObjectTypeQuery3") "/Game/Blueprints/AI.AI_C" (Utilities|Array|MakeArray (Pawn|GetControlledPawn))))
  (if _returnvalue
    (for _array_element _outactors
      (bind _asai (Utilities|Casting|CastToAI _array_element)
        (:then
          (bind _asai_2 (Utilities|Casting|CastToAI (Pawn|GetControlledPawn))
            (:then
              (if (Variables|/Game/Blueprints/AI.AI_C|GetInfected _asai)
                (if (Variables|/Game/Blueprints/AI.AI_C|GetInfected _asai_2)
                  (Development|PrintString "Both infected, do nothing!")
                  (else
                    (CallFunction|SpawnDiseaseSpread _asai_2)
                    (Variables|/Game/Blueprints/AI.AI_C|SetInfected _asai_2 true)))
                (elif (not (Variables|/Game/Blueprints/AI.AI_C|GetInfected _asai_2))
                  (Development|PrintString "None is infected"))))
            (:CastFailed
              (Development|PrintString "Cast failed" :!label _label))))
        (:CastFailed
          (goto _label))))))

(event EventBeginPlay
  (Utilities|FlowControl|Sequence
    (:then_0
      (bind _outactors (Actor|GetAllActorsOfClass "/Script/Engine.RecastNavMesh"))
      (for _array_element _outactors
        _))
    (:then_1
      (CallFunction|SpawnFirstDisease))))

(event EventOnPossess
  (params (PossessedPawn :type Pawn%20Object%20Reference))
  ;[1 1 1] Initialize AI
)

(fn ConstructionScript)

(fn MovetoRandomLocation
  (params (Nav%20Data :type Recast%20Nav%20Mesh%20Object%20Reference))
  (bind _ascharacter (Utilities|Casting|CastToCharacter (Pawn|GetControlledPawn)))
  (if (>= (Math|Vector|VectorLength (- (Transformation|GetActorLocation _ascharacter) (Class|NavigationSystem|GetRandomPointinRadius (Transformation|GetActorLocation _ascharacter) 5e+03 Nav%20Data))) 1e+03)
    (bind _returnvalue (AI|Navigation|MovetoLocation (Variables|Default|GetNew%20destination) -1.0 true true false true))
    (switch Utilities|FlowControl|Switch|SwitchonEPathFollowingRequestResult _returnvalue
      (:Failed
        _)
      (:AlreadyAtGoal
        _))
    (Variables|Default|SetNew%20destination (Class|NavigationSystem|GetRandomPointinRadius (Transformation|GetActorLocation _ascharacter) 5e+03 Nav%20Data))))

(fn GetCharacterLocation
  (bind _ascharacter (Utilities|Casting|CastToCharacter (Pawn|GetControlledPawn)))
  (return (Transformation|GetActorLocation _ascharacter)))

(fn SpawnFirstDisease
  (bind _asai (Utilities|Casting|CastToAI (Pawn|GetControlledPawn))
    (:then
      (if (Variables|/Game/Blueprints/AI.AI_C|GetInfected _asai)
        (Effects|SpawnEmitterAttached "/Game/Blueprints/Particals/P_disease.P_disease" (Variables|/Script/Engine.Character|GetMesh _asai) "None")))
    (:CastFailed
      _))
  (return))

(fn SpawnDiseaseSpread
  (params (Object :type Object%20Object%20Reference))
  (bind _asai (Utilities|Casting|CastToAI Object)
    (:then
      (if (Variables|/Game/Blueprints/AI.AI_C|GetInfected _asai)
        _
        (else
          (Effects|SpawnEmitterAttached "/Game/Blueprints/Particals/P_disease.P_disease" (Variables|/Script/Engine.Character|GetMesh _asai) "None"))))
    (:CastFailed
      _))
  (return))

(fn SetRelation
  (bind _outactors (Actor|GetAllActorsOfClass "/Game/Blueprints/AI.AI_C"))
  (for (_array_element _array_index) _outactors
    (if (<= _array_index 0)
      (Variables|/Game/Blueprints/AI.AI_C|SetRelation _array_element "Init"))
    (return))
  (return))